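; BP_Enemy is an enemy Blueprint that shows its health on an HP widget and destroys itself when health runs out.
; OnHealthChanged prints the current health, then casts the HPWidget's user widget to WBP_EnemyHP and sets its progress to health over max health.
; The zero-health check runs only after that cast succeeds.
; BeginPlay, overlap, Tick and the construction script are empty.
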(event `self.ReceiveBeginPlay`)

(event `self.OnHealthChanged`
  (params (DeltaValue :type "Float (single-precision)") (EventTags :type "GameplayTagContainer Structure (by ref)"))
  (bind _returnvalue (`self.GetHealth`))
  (`KismetSystemLibrary.PrintString` (`KismetStringLibrary.Conv_DoubleToString` _returnvalue))
  (bind _aswbp_enemy_hp (cast `/Game/Blueprints/WidgetBP/WBP_EnemyHP` (`WidgetComponent.GetUserWidgetObject` (`self.HP_Widget`))))
  (`/Game/Blueprints/WidgetBP/WBP_EnemyHP.SetProgress` _aswbp_enemy_hp (/ _returnvalue (`self.GetMaxHealth`)))
  (if (<= (`self.GetHealth`) 0.0)
    (`self.K2_DestroyActor`)))

(fn `UserConstructionScript`)