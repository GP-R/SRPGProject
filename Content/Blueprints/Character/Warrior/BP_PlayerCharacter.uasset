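; Warrior player character Blueprint whose Attack event plays a dialogue.
; Attack casts player controller 0 to BP_PlayerController and has its dialogue controller play AttackDialogue with movement allowed.
; A disconnected, never-executed branch sphere-overlaps enemies at the sword_top socket and sends a Weapon.Hit gameplay event to the instigator, targeting the first hit.
; BeginPlay, Tick, overlap and construction logic are empty.
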(event `self.ReceiveBeginPlay`)

(event `self.ReceiveTick`
  (params (DeltaSeconds :type "Float (single-precision)")))

(event `Attack`
  (bind _asbp_player_controller (cast `/Game/Blueprints/BP_PlayerController` (`GameplayStatics.GetPlayerController` 0)))
  (bind _returnvalue (`SRPGPlayerController.GetDialogueController` _asbp_player_controller))
  (`DialogueController.PlayDialogue` _returnvalue (`self.AttackDialogue`) true))

(fn `UserConstructionScript`)