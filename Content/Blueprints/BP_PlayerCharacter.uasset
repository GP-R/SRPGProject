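; BP_PlayerCharacter is the player character Blueprint, handling sword hit detection for melee attacks through the Gameplay Ability System.
; Its Attack event runs a small sphere overlap at the sword_top mesh socket, looking for BP_Enemy pawns while ignoring itself.
; The first enemy found is sent as target data in a Weapon.Hit gameplay event to the instigator.
; BeginPlay, Tick, overlap and construction logic are empty.
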(event `self.ReceiveBeginPlay`)

(event `self.ReceiveTick`
  (params (DeltaSeconds :type "Float (single-precision)")))

(event `Attack`
  (bind _returnvalue (`self.GetInstigator`))
  (bind _outactors (`KismetSystemLibrary.SphereOverlapActors` (`SceneComponent.GetSocketLocation` (`self.Mesh`) "sword_top") 50.0 (`|MakeArray` "ObjectTypeQuery3" :!type "EObjectTypeQuery Enum") "/Game/Blueprints/BP_Enemy.BP_Enemy_C" (`|MakeArray` self :!type "Actor Object Reference")))
  (if (`KismetArrayLibrary.Array_IsValidIndex` _outactors)
    (bind _output (`|GetArrayItem` _outactors))
    (`AbilitySystemBlueprintLibrary.SendGameplayEventToActor` _returnvalue (struct :`TagName` "Weapon.Hit") (make `GameplayEventData` (struct) _returnvalue _output null null (struct) (struct) (struct) 0.0 (`AbilitySystemBlueprintLibrary.AbilityTargetDataFromActor` _output)))))

(fn `UserConstructionScript`)